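; Base AI controller for turtle pawns that starts their behavior and seeds its movement data.
; On possession it casts the pawn to BP_Turtle and runs that turtle's own behavior tree.
; It then writes the turtle's destination and its current location, as the spawn point, into the Blackboard for the tree to use.
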(event `self.ReceivePossess`
  (params (PossessedPawn :type "Pawn Object Reference"))
  ;[1 1 1] Run BT and Set Start/Destination locations
  (bind _asbp_turtle (cast `/Game/Turtles/Blueprints/BP_Turtle` PossessedPawn))
  (`self.RunBehaviorTree` (`/Game/Turtles/Blueprints/BP_Turtle.BehaviorTree` _asbp_turtle))
  (`BlackboardComponent.SetValueAsVector` (`self.Blackboard`) "DestinationLocation" (`/Game/Turtles/Blueprints/BP_Turtle.DestinationLocation` _asbp_turtle))
  (`BlackboardComponent.SetValueAsVector` (`self.Blackboard`) "SpawnLocation" (`self.K2_GetActorLocation` _asbp_turtle)))

(fn `UserConstructionScript`)