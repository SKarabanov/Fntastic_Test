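; BP_Button is an interactable scene button that shows its ButtonName on a text label set at construction.
; Its Box overlap tells actors implementing BPI_Interaction when they enter or leave range, so they can show an interaction message.
; Interact starts the ButtonPushing timeline unless it is already playing.
; The timeline animates the button's press along Z and fires the OnInteraction dispatcher from an event track for listeners.
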(event `self.Box.OnComponentBeginOverlap`
  (params (OverlappedComponent :type "PrimitiveComponent Object Reference") (OtherActor :type "Actor Object Reference") (OtherComp :type "PrimitiveComponent Object Reference") (OtherBodyIndex :type Integer) (bFromSweep :type Boolean) (SweepResult :type "HitResult Structure (by ref)"))
  ;[1 1 1] Show interaction message when overlapped
  (if (`KismetSystemLibrary.DoesImplementInterface` OtherActor "/Game/Turtles/Blueprints/BPI_Interaction.BPI_Interaction_C")
    (message `/Game/Turtles/Blueprints/BPI_Interaction.InteractionOverlap` OtherActor true self)))

(event `self.Box.OnComponentEndOverlap`
  (params (OverlappedComponent :type "PrimitiveComponent Object Reference") (OtherActor :type "Actor Object Reference") (OtherComp :type "PrimitiveComponent Object Reference") (OtherBodyIndex :type Integer))
  ;[1 1 1] Show interaction message when overlapped
  (if (`KismetSystemLibrary.DoesImplementInterface` OtherActor "/Game/Turtles/Blueprints/BPI_Interaction.BPI_Interaction_C")
    (message `/Game/Turtles/Blueprints/BPI_Interaction.InteractionOverlap` OtherActor false self)))

(event `/Game/Turtles/Blueprints/BPI_Interaction.Interact`
  ;[1 1 1] Interaction
  (if (not (`TimelineComponent.IsPlaying` (`self.ButtonPushing`)))
    (`TimelineComponent.PlayFromStart` (`self.ButtonPushing`))))

(fn `InteractionOverlap`
  (params (Overlapped :type Boolean) (Actor :type "Actor Object Reference"))
  (returns (Success :type Boolean))
  (return false))

(fn `UserConstructionScript`
  (`TextRenderComponent.K2_SetText` (`self.TextRender`) (`self.ButtonName`)))