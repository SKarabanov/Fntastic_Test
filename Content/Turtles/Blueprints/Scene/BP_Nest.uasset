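; BP_Nest is an interactable turtle nest that spawns a turtle and sends it toward a finish point.
; On Interact it replaces any previous turtle with a new BP_Turtle at SceneStart, passing a behavior tree and SceneFinish as the destination.
; When that turtle overlaps the Sphere, it is destroyed with a finish effect.
; Start and finish effects spawn as BP_EffectActor, snapped to WorldStatic ground by a vertical line trace.
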(event `/Game/Turtles/Blueprints/BPI_Interaction.Interact`
  ;[1 1 1] On interaction
  (`self.SpawnTurtle`)
  (`self.SpawnVFX` (`SceneComponent.K2_GetComponentLocation` (`self.SceneStart`)) "/Game/Turtles/Particles/Start/P_OncomingLines.P_OncomingLines"))

(event `self.Sphere.OnComponentBeginOverlap`
  (params (OverlappedComponent :type "PrimitiveComponent Object Reference") (OtherActor :type "Actor Object Reference") (OtherComp :type "PrimitiveComponent Object Reference") (OtherBodyIndex :type Integer) (bFromSweep :type Boolean) (SweepResult :type "HitResult Structure (by ref)"))
  ;[1 1 1] On finish overlap
  (bind _spawnedturtle (`self.SpawnedTurtle`)
    (:`then`
      (if (== _spawnedturtle OtherActor)
        (`self.SpawnVFX` (`SceneComponent.K2_GetComponentLocation` (`self.SceneFinish`)) "/Game/Turtles/Particles/Finish/P_Qusar.P_Qusar")
        (`self.K2_DestroyActor` (`self.SpawnedTurtle`))))
    (:`else`)))

(fn `ClearTurtle`
  (bind _spawnedturtle (`self.SpawnedTurtle`)
    (:`then`
      (`self.K2_DestroyActor` _spawnedturtle))
    (:`else`)))

(fn `InteractionOverlap`
  (params (Overlapped :type Boolean) (Actor :type "Actor Object Reference"))
  (returns (Success :type Boolean))
  (return false))

(fn `SpawnTurtle`
  (bind (_returnvalue_location _returnvalue_rotation) (`KismetMathLibrary.BreakTransform` (`SceneComponent.K2_GetComponentToWorld` (`self.SceneStart`))))
  (`self.ClearTurtle`)
  (bind _returnvalue (`|SpawnActorFromClass` "/Game/Turtles/Blueprints/BP_Turtle.BP_Turtle_C" (`KismetMathLibrary.MakeTransform` _returnvalue_location _returnvalue_rotation) "AlwaysSpawn" "OverrideRootScale" null (`self.BehaviorTree`) (`SceneComponent.K2_GetComponentLocation` (`self.SceneFinish`)) null))
  (set `self.SpawnedTurtle` _returnvalue))

(fn `SpawnVFX`
  (params (Location :type "Vector Structure") (Particle :type "ParticleSystem Object Reference"))
  (bind (_outhit _returnvalue) (`KismetSystemLibrary.LineTraceSingleForObjects` (+ Location (0.0 0.0 100.0)) (+ Location (0.0 0.0 -500.0)) (`|MakeArray` "ObjectTypeQuery1" :!type "EObjectTypeQuery Enum")))
  (if _returnvalue
    (`|SpawnActorFromClass` "/Game/Turtles/Blueprints/BP_EffectActor.BP_EffectActor_C" (`KismetMathLibrary.Conv_VectorToTransform` (`.Location` (`GameplayStatics.BreakHitResult` _outhit))) "AlwaysSpawn" "OverrideRootScale" null (`local.Particle`) null)))

(fn `UserConstructionScript`)