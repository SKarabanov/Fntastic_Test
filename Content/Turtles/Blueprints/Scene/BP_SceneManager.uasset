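; BP_SceneManager is a scene manager that relays interactions from controller actors to the actors they control.
; On BeginPlay it binds an event to the OnInteraction dispatcher of each valid entry in ControllerActors.
; InteriorInteraction looks up an actor's index in ControllerActors and calls InteractMessage on the ControlledActors entry at the same index.
; The two parallel arrays define the pairings, so their order determines which controller triggers which actor.
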(event `self.ReceiveBeginPlay`
  (for _array_element (`self.ControllerActors`)
    (`/Engine/EditorBlueprintResources/StandardMacros.IsValid` _array_element
      (:`Is Valid`
        (add `/Game/Turtles/Blueprints/Scene/BP_SceneControllerBase.OnInteraction` _array_element (`|CreateDelegate` :!event `InteriorInteraction`))))))

(fn `InteriorInteraction`
  (params (Actor :type "/Game/Turtles/Blueprints/Scene/BP_SceneControllerBase Object Reference"))
  (if (`KismetArrayLibrary.Array_Contains` (`self.ControllerActors`) Actor)
    (if (`KismetArrayLibrary.Array_IsValidIndex` (`self.ControlledActors`) (`KismetArrayLibrary.Array_Find` (`self.ControllerActors`) Actor))
      (message `/Game/Turtles/Blueprints/BPI_Interaction.Interact` (`|GetArrayItem` (`self.ControlledActors`) (`KismetArrayLibrary.Array_Find` (`self.ControllerActors`) (`local.Actor`)))))))

(fn `UserConstructionScript`)